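; Health pickup Blueprint that restores the collecting character to full health.
; It overrides Pickup to set the character's health to its MaxHealth, guarded by a validity check on the static mesh.
; Deactivate and reactivate overrides call the parent logic, then hide or show the mesh.
; The event graph holds only disabled placeholder events, so this Blueprint adds no overlap or tick logic.
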(fn `OnDeactivate`
  (`parent.OnDeactivate`)
  (`SceneComponent.SetVisibility` (`self.StaticMesh`) false false))

(fn `OnReactivate`
  (`parent.OnReactivate`)
  (`SceneComponent.SetVisibility` (`self.StaticMesh`) true false))

(fn `Pickup`
  (params (Character :type "/Game/MyContent/Characters/BP_Character Object Reference"))
  (`self.StaticMesh`
    (:`then`
      (`/Game/MyContent/Characters/BP_Character.Set Health` Character (`/Game/MyContent/Characters/BP_Character.MaxHealth` Character)))
    (:`else`)))

(fn `UserConstructionScript`
  (`parent.UserConstructionScript`))