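; Grenade round projectile that explodes when its Box component begins an overlap.
; On overlap it queries Pawn and Destructible actors within the Sphere component's scaled radius and applies point damage to each, crediting the instigator's controller.
; It destroys itself inside the damage loop, then calls DestroyGrenadeProjectile to spawn the explosion particle and destroy the actor.
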(event `self.Box.OnComponentBeginOverlap`
  (params (OverlappedComponent :type "PrimitiveComponent Object Reference") (OtherActor :type "Actor Object Reference") (OtherComp :type "PrimitiveComponent Object Reference") (OtherBodyIndex :type Integer) (bFromSweep :type Boolean) (SweepResult :type "HitResult Structure (by ref)"))
  (bind _outactors (`KismetSystemLibrary.SphereOverlapActors` (`self.K2_GetActorLocation`) (`SphereComponent.GetScaledSphereRadius` (`self.Sphere`)) (`|MakeArray` "ObjectTypeQuery3" "ObjectTypeQuery6" :!type "EObjectTypeQuery Enum") null (`|MakeArray` self :!type "Actor Object Reference")))
  (for _array_element _outactors
    (`GameplayStatics.ApplyPointDamage` _array_element (`self.Damage`) (`self.GetActorForwardVector`) (`GameplayStatics.MakeHitResult` false) (`self.GetInstigatorController`) self)
    (`self.K2_DestroyActor`))
  (`self.DestroyGrenadeProjectile`))

(fn `DestroyGrenadeProjectile`
  (`GameplayStatics.SpawnEmitterAtLocation` "/Game/MilitaryWeapDark/FX/P_Grenade_Explosion_01.P_Grenade_Explosion_01" (`self.K2_GetActorLocation`))
  (`self.K2_DestroyActor`))

(fn `UserConstructionScript`)