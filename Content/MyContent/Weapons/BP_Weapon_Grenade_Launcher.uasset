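; Grenade launcher weapon Blueprint, a child weapon class that fires grenade projectiles.
; Its damage activation delegates to the owning character's grenade-shooting function, leaving the passed shot location and direction unused.
; The multicast fire animation plays weapon and character montages, with play rates set to the inverse of the fire rate.
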(event `self.Multi_AnimFire`
  (`AnimInstance.Montage_Play` (`SkeletalMeshComponent.GetAnimInstance` (`self.SKM_Weapon`)) (`self.Fire_Weapon`) (/ 1.0 (`self.FireRate`)) "Duration" 0.0 true)
  (`self.PlayCharacterMontage` (`self.Fire_Character`) (/ 1.0 (`self.FireRate`))))

(fn `ActivateDamage`
  (params (ShootLoc :type "Vector Structure") (ShootDir :type "Vector Structure"))
  (`/Game/MyContent/Characters/BP_Character.ProjectileShootGrenade` (`self.CharcterOwner`)))

(fn `UserConstructionScript`
  (`parent.UserConstructionScript`))