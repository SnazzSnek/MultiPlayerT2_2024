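; Shotgun weapon Blueprint that fires several line-damage pellets per shot.
; On BeginPlay it divides Damage by BulletsPerShot, splitting the shot's damage evenly across pellets.
; ActivateDamage calls ApplyLineDamage per pellet in a random cone direction, with the cone half-angle growing by pellet index, so the first goes straight and later ones can stray toward SpreadAngle.
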(event `self.ReceiveBeginPlay`
  (set `self.Damage` (/ (`self.Damage`) (`self.BulletsPerShot`))))

(fn `ActivateDamage`
  (params (ShootLoc :type "Vector Structure") (ShootDir :type "Vector Structure"))
  (bind _bulletspershot (`self.BulletsPerShot`))
  (for _index (range _bulletspershot)
    (`self.Apply Line Damage` (`local.ShootLoc`) (`KismetMathLibrary.RandomUnitVectorInConeInDegrees` (`local.ShootDir`) (* _index (/ (`self.SpreadAngle`) _bulletspershot))))))

(fn `UserConstructionScript`
  (`parent.UserConstructionScript`))